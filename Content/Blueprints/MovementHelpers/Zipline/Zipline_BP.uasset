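; Zipline actor that carries the player along a spline when Jump is pressed inside its Start trigger.
; The construction script builds spline mesh segments along the Zipline spline and positions Start and End from its points.
; Start overlaps toggle the actor's input, and Jump plays a DoOnce-gated timeline that moves the player with sweep through NewLoc.
; Player jumping is disabled during the ride and restored on finish.
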(event OnComponentBeginOverlap(Start)
  (params (OverlappedComponent :type Primitive%20Component%20Object%20Reference) (OtherActor :type Actor%20Object%20Reference) (OtherComp :type Primitive%20Component%20Object%20Reference) (OtherBodyIndex :type Integer) (bFromSweep :type Boolean) (SweepResult :type Hit%20Result%20Structure%20%28by%20ref%29))
  ;[1 1 1] Toggle Input
  (Utilities|Casting|CastToPlayerCharacter OtherActor)
  (Input|EnableInput (Game|GetPlayerController 0)))

(event OnComponentEndOverlap(Start)
  (params (OverlappedComponent :type Primitive%20Component%20Object%20Reference) (OtherActor :type Actor%20Object%20Reference) (OtherComp :type Primitive%20Component%20Object%20Reference) (OtherBodyIndex :type Integer))
  ;[1 1 1] Toggle Input
  (Utilities|Casting|CastToPlayerCharacter OtherActor)
  (Input|DisableInput (Game|GetPlayerController 0)))

(event Custom|Reset
  ;[1 1 1] Zipline Movement
  (Variables|/Game/ThirdPersonBP/Blueprints/PlayerCharacter.PlayerCharacter_C|SetCanJump? (Variables|Default|GetPlayer) true)
  (Utilities|FlowControl|DoOnce false) ; enters at Reset
)

(event EventBeginPlay
  ;[1 1 1] BeginPlay
  (bind _asplayer_character (Utilities|Casting|CastToPlayerCharacter (Game|GetPlayerCharacter 0)))
  (Variables|Default|SetPlayer _asplayer_character)
  (Components|Timeline|SetPlayRate (Variables|Default|GetZipTime) (Variables|Default|GetPlayRate)))

(event Input|ActionEvents|InputActionJump
  (params (Key :type Key%20Structure))
  ;[1 1 1] Zipline Movement
  (:Pressed
    (Variables|/Game/ThirdPersonBP/Blueprints/PlayerCharacter.PlayerCharacter_C|SetCanJump? (Variables|Default|GetPlayer) false)
    (Utilities|FlowControl|DoOnce false
      (:Completed
        (bind _movement (Timeline|ZipTime PlayFromStart)
          (:Update
            (Transformation|SetActorLocation (Variables|Default|GetPlayer) (Utilities|NewLoc _movement) true false))
          (:Finished
            (CallFunction|Reset)))))))

(fn ConstructionScript
  (bind _zipline (Variables|Default|GetZipline))
  (bind _zipline_2 (Variables|Default|GetZipline))
  (bind _returnvalue (Spline|GetNumberOfSplinePoints _zipline))
  (for _index (range 0 (- _returnvalue 2))
    ;[1 1 1] Ser Start and End Points
    (Transformation|SetRelativeLocation (Variables|Default|GetStart) (.Location (Spline|GetLocationandTangentatSplinePoint _zipline_2 (Utilities|Array|Get(acopy) (Utilities|Array|MakeArray _returnvalue) _returnvalue) "Local")) false false)
    (Transformation|SetRelativeLocation (Variables|Default|GetEnd) (.Location (Spline|GetLocationandTangentatSplinePoint _zipline_2 (Utilities|Array|Get(acopy) (Utilities|Array|MakeArray _returnvalue)) "Local")) false false)
    (bind _returnvalue_2 (AddComponent|AddSplineMeshComponent false))
    (Transformation|AttachComponentToComponent (Variables|Default|GetDefaultSceneRoot) _returnvalue_2 "None" "KeepRelative" "KeepRelative" "KeepRelative" true)
    (SplineMesh|SetStartandEnd _returnvalue_2 (.Location (Spline|GetLocationandTangentatSplinePoint (Variables|Default|GetZipline) _index "Local")) (.Tangent (Spline|GetLocationandTangentatSplinePoint (Variables|Default|GetZipline) _index "Local")) (.Location (Spline|GetLocationandTangentatSplinePoint (Variables|Default|GetZipline) (+ _index 1) "Local")) (.Tangent (Spline|GetLocationandTangentatSplinePoint (Variables|Default|GetZipline) (+ _index 1) "Local")) true :!class /Script/Engine.SplineMeshComponent)))